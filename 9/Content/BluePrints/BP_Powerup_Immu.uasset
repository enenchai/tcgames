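; BP_Powerup_Immu is a powerup that acts as immunity by refilling the affected actor's health while active.
; Activation stores the actor's current SHealthComponent health in ThisHealth, which these graphs never read back.
; Each update sets CurrentHealth directly to DefaultHealth, so damage is undone on update rather than blocked.
; The mesh hides while the powerup is active, and the actor destroys itself on expiry.
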(event EventOnUpdated
  (Variables|/Script/s1116.SHealthComponent|SetCurrentHealth (Actor|GetComponentbyClass (stale EventOnActived OtherActor) "/Script/s1116.SHealthComponent") (Variables|/Script/s1116.SHealthComponent|GetDefaultHealth (Actor|GetComponentbyClass (stale EventOnActived OtherActor) "/Script/s1116.SHealthComponent"))))

(event EventOnActived
  (params (OtherActor :type Actor%20Object%20Reference))
  (Variables|Default|SetThisHealth (Variables|/Script/s1116.SHealthComponent|GetCurrentHealth (Actor|GetComponentbyClass OtherActor "/Script/s1116.SHealthComponent"))))

(event EventOnExpired
  (Actor|DestroyActor))

(event EventOnPowerupStateChanged
  (params (bNewActive :type Boolean))
  (Rendering|SetVisibility (Variables|Default|GetStaticMesh) (not bNewActive) false))

(fn ConstructionScript)