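; BP_Powerup_Recover is a powerup that restores health to the actor that activates it.
; It stores that actor on activation, then calls Heal on its SHealthComponent with HealAmount at each powerup update while the actor remains valid.
; The static mesh hides while the powerup is active, and the actor destroys itself when the powerup expires.
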(event EventOnActived
  (params (OtherActor :type Actor%20Object%20Reference) (ThisWeapon :type S%20Weapon%20Object%20Reference))
  (Variables|Default|SetOtherActor OtherActor))

(event EventOnUpdated
  (Utilities|IsValid (Variables|Default|GetOtherActor)
    (:Is%20Valid
      (Class|SHealthComponent|Heal (Actor|GetComponentbyClass (stale EventOnActived OtherActor) "/Script/s1116.SHealthComponent") (Variables|Default|GetHealAmount)))))

(event EventOnExpired
  (Actor|DestroyActor))

(event EventOnPowerupStateChanged
  (params (bNewActive :type Boolean))
  (Rendering|SetVisibility (Variables|Default|GetStaticMesh) (not bNewActive) false))

(fn ConstructionScript)