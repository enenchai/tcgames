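; BP_AdvancedAI is an AI-controlled actor that hands its behavior to the BT_AdvancedAI behavior tree.
; On BeginPlay it runs the tree through its AI controller, then seeds the TargetD blackboard key with a hardcoded vector.
; A disconnected node that would store the player pawn as TargetActor never runs, so this Blueprint does not set that key.
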(event EventBeginPlay
  (AI|RunBehaviorTree (AI|GetAIController self) "/Game/BluePrints/BT_AdvancedAI.BT_AdvancedAI")
  (AI|Components|Blackboard|SetValueasVector (AI|GetBlackboard self) (Utilities|Name|MakeLiteralName "TargetD") "0, 0,88.000000"))

(fn ConstructionScript)