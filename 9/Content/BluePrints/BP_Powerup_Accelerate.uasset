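; Accelerate powerup that boosts the affected actor's movement speed, jump, weapon damage and damage immunity rate.
; The state-change event toggles mesh visibility and applies the boosts regardless of the new state, using actor and weapon references from the otherwise empty OnActived event.
; OnExpired calls DestroyActor, then divides movement values back and sets fixed damage and immunity values.
; BeginPlay also runs the immunity write, without an activation supplying the actor.
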(event EventBeginPlay
  (Variables|/Script/s1116.SHealthComponent|SetImmuneRate (Actor|GetComponentbyClass (stale EventOnActived OtherActor) "/Script/s1116.SHealthComponent") 0.01))

(event EventOnExpired
  (Actor|DestroyActor)
  (Variables|/Script/Engine.CharacterMovementComponent|SetMaxWalkSpeed (Actor|GetComponentbyClass (stale EventOnActived OtherActor) "/Script/Engine.CharacterMovementComponent") (/ (Class|MovementComponent|GetMaxSpeed (Actor|GetComponentbyClass (stale EventOnActived OtherActor) "/Script/Engine.CharacterMovementComponent")) 2.0))
  (Variables|/Script/Engine.CharacterMovementComponent|SetJumpZVelocity (Actor|GetComponentbyClass (stale EventOnActived OtherActor) "/Script/Engine.CharacterMovementComponent") (/ (Variables|/Script/Engine.CharacterMovementComponent|GetJumpZVelocity (Actor|GetComponentbyClass (stale EventOnActived OtherActor) "/Script/Engine.CharacterMovementComponent")) 1.4))
  (Variables|/Script/s1116.SWeapon|SetBaseDamage (stale EventOnActived ThisWeapon) 2e+01)
  (Variables|/Script/s1116.SHealthComponent|SetImmuneRate (Actor|GetComponentbyClass (stale EventOnActived OtherActor) "/Script/s1116.SHealthComponent") 1.0))

(event EventOnActived
  (params (OtherActor :type Actor%20Object%20Reference) (ThisWeapon :type S%20Weapon%20Object%20Reference)))

(event EventOnPowerupStateChanged
  (params (bNewActive :type Boolean))
  (Rendering|SetVisibility (Variables|Default|GetStaticMesh) (not bNewActive) false)
  (Variables|/Script/Engine.CharacterMovementComponent|SetMaxWalkSpeed (Actor|GetComponentbyClass (stale EventOnActived OtherActor) "/Script/Engine.CharacterMovementComponent") (* (Class|MovementComponent|GetMaxSpeed (Actor|GetComponentbyClass (stale EventOnActived OtherActor) "/Script/Engine.CharacterMovementComponent")) 2.0))
  (Variables|/Script/Engine.CharacterMovementComponent|SetJumpZVelocity (Actor|GetComponentbyClass (stale EventOnActived OtherActor) "/Script/Engine.CharacterMovementComponent") (* (Variables|/Script/Engine.CharacterMovementComponent|GetJumpZVelocity (Actor|GetComponentbyClass (stale EventOnActived OtherActor) "/Script/Engine.CharacterMovementComponent")) 1.4))
  (Variables|/Script/s1116.SWeapon|SetBaseDamage (stale EventOnActived ThisWeapon) 1e+02)
  (Variables|/Script/s1116.SHealthComponent|SetImmuneRate (Actor|GetComponentbyClass (stale EventOnActived OtherActor) "/Script/s1116.SHealthComponent") 0.01))

(fn ConstructionScript)